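; BP_Plan is a textured plane actor, likely a plan image in the viewer, that can be repositioned with the mouse.
; SetUpPlan scales the plane from the given size and applies the texture through a dynamic material instance.
; When Move is set, clicks spawn a BP_Origin at the cursor hit and alternate between attaching the plan to it and detaching.
; While attached, a gated Tick moves that origin to the cursor hit, carrying the plan along.
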(event `self.ReceiveTick`
  (params (DeltaSeconds :type "Float (single-precision)"))
  (`/Engine/EditorBlueprintResources/StandardMacros.Gate` true :!label _label
    (:`Exit`
      (`self.K2_SetActorLocation` (`self.Origin`) (`.Location` (`GameplayStatics.BreakHitResult` (`PlayerController.GetHitResultUnderCursorForObjects` (`GameplayStatics.GetPlayerController` 0) (`|MakeArray` "ObjectTypeQuery1" "ObjectTypeQuery2" :!type "EObjectTypeQuery Enum") true))) false false))))

(event `self.Plane.OnClicked`
  (params (TouchedComponent :type "PrimitiveComponent Object Reference") (ButtonPressed :type "Key Structure"))
  (if (`self.bMove`)
    (bind _returnvalue (`|SpawnActorFromClass` "/Game/Viewer/01_Core/Plan/BP_Origin.BP_Origin_C" (`KismetMathLibrary.MakeTransform` (`.Location` (`GameplayStatics.BreakHitResult` (`PlayerController.GetHitResultUnderCursorByChannel` (`GameplayStatics.GetPlayerController` 0) "TraceTypeQuery1" true)))) "Undefined" "OverrideRootScale" null null))
    (set `self.Origin` _returnvalue)
    (`|MultiGate` false true
      (:`Out 0`
        (`self.K2_AttachToActor` (`self.Origin`) "None" "KeepWorld" "KeepWorld" "KeepWorld")
        (goto _label :!via `Open`))
      (:`Out 1`
        (set `self.bMove` false)
        (`self.K2_DetachFromActor` "KeepWorld" "KeepWorld" "KeepWorld")
        (`self.K2_DestroyActor` (`self.Origin`))
        (goto _label :!via `Close`)))))

(fn `SetUpPlan`
  (params (SizeX :type Integer) (SizeY :type Integer) (Texture :type "Texture2D Object Reference"))
  (bind _plane (`self.Plane`))
  (`SceneComponent.SetRelativeScale3D` (`self.Plane`) (`KismetMathLibrary.MakeVector` (/ (`KismetMathLibrary.Conv_IntToDouble` SizeX) 10.0) (/ (`KismetMathLibrary.Conv_IntToDouble` SizeY) 10.0) 1.0))
  (bind _returnvalue (`PrimitiveComponent.CreateDynamicMaterialInstance` _plane 0 (`PrimitiveComponent.GetMaterial` _plane 0) "None"))
  (`MaterialInstanceDynamic.SetTextureParameterValue` _returnvalue "Texture" (`local.Texture`))
  (`PrimitiveComponent.SetMaterial` (`self.Plane`) 0 _returnvalue))

(fn `UserConstructionScript`)