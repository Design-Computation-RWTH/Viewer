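; Viewer game mode that holds the entry points for importing IFC files.
; ImportFile removes the first logo actor, opens a file dialog, logs the import and stores the chosen name and path.
; Separate ImportIfc and ParseIfc functions each add a geometry or parser component at runtime and call its ConvertIfc directly.
; ImportFile does not call either one, and its own property-parsing branch is disconnected.
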(fn `Import File`
  (params (DialogTitle :type String) (FileTypes :type String) (bAdd :type Boolean))
  (locals (LastImport :type "Object Object Reference") (FileName :type String) (FilePath :type String))
  ;[1 1 1] Loop through the imported elements and create viewerActor for it.
  (bind _outactors (`GameplayStatics.GetAllActorsOfClass` "/Game/Viewer/03_Art/DC/BP_DC_Logo.BP_DC_Logo_C"))
  (if (`KismetArrayLibrary.Array_IsValidIndex` _outactors)
    (`self.K2_DestroyActor` (`|GetArrayItem` _outactors)))
  (bind (_name _path) (`/Game/Viewer/01_Core/ViewerBlueprints.ImportFile` DialogTitle FileTypes "C:/" bAdd))
  (`self.EventLog` "Importing IFC")
  (if (not (`KismetStringLibrary.IsEmpty` _name))
    (set `local.FileName` _name)
    (set `local.FilePath` _path)))

(fn `ImportIfc`
  (params (FileName :type String) (FilePath :type String))
  (bind _returnvalue (`AddComponent|NODE_AddABP_IfcGeometrie-0` :`FileName` FileName :`FilePath` FilePath))
  (`/Game/Viewer/01_Core/IfcGeometrie/ABP_IfcGeometrie.ConvertIfc` _returnvalue FileName FilePath))

(fn `ParseIfc`
  (params (FileName :type String) (FilePath :type String))
  (bind _returnvalue (`AddComponent|NODE_AddABP_IfcParser-2` :`FileName` FileName :`FilePath` FilePath))
  (`/Game/Viewer/01_Core/IfcParse/ABP_IfcParser.ConvertIfc` _returnvalue))

(fn `UserConstructionScript`)