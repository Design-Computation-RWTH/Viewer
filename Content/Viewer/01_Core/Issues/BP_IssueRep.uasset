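; Actor representing a filtered issue in the 3D viewer, placed at its first viewpoint's transform on BeginPlay.
; Clicking its camera marker selects the issue's widget and scrolls it into view; ShowHide toggles marker visibility and collision.
; LineTraceForPixels scales a plane to a hardcoded pixel resolution, then steps a helper across it to aim one trace per pixel from the Arrow.
; Hit ViewerMeshActors are collected uniquely into VisibleActors.
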(event `self.ReceiveBeginPlay`
  (bind _issue (`/BcfCommunication/Library/BcfFunctionLibrary.GetFilteredIssue` (`self.IssueIndex`)))
  (`self.K2_SetActorTransform` (`/BcfCommunication/Library/BcfFunctionLibrary.GetViewpointTransform` (`|GetArrayItem` (`.Viewpoints` (break `MarkupStruct` _issue))))))

(event `self.Camera.OnClicked`
  (params (TouchedComponent :type "PrimitiveComponent Object Reference") (ButtonPressed :type "Key Structure"))
  (bind _widget (`self.Widget`))
  (`/CAIAViewer/UI/Panels/Topics/WBP_TopicPreview.Select` _widget)
  (`ScrollBox.ScrollWidgetIntoView` (`/CAIAViewer/UI/Panels/Topics/WBP_Topics.SB_Topics` (`self.TopicWidget`)) _widget true "IntoView" 0.0))

(fn `CalculatePixelDensity`
  (params (Width :type Integer) (Height :type Integer)))

(fn `CalculateStartAndEndPoint`
  (params (Point :type "Vector Structure (by ref)"))
  (returns (Start :type "Vector Structure") (End :type "Vector Structure"))
  (bind _mylittehelper (`self.MyLitteHelper`))
  (bind _returnvalue (`SceneComponent.K2_GetComponentLocation` (`self.Arrow`)))
  (`SceneComponent.K2_SetRelativeLocation` _mylittehelper Point false false)
  (return _returnvalue (+ _returnvalue (* (`KismetMathLibrary.GetForwardVector` (`KismetMathLibrary.FindLookAtRotation` _returnvalue (`SceneComponent.K2_GetComponentLocation` _mylittehelper))) 5000.0))))

(fn `LineTraceForPixels`
  (locals (Image :type "Texture2D Object Reference") (FovW :type "Float (double-precision)") (FovH :type "Float (double-precision)") (PixelWidth :type Integer :default 0) (PixelHeight :type Integer :default 0) (Test :type Integer) (NextPoint :type "Vector Structure" :default (0.0 0.0 0.0)) (LoopIndex :type Integer))
  (bind (_start _end) (`self.CalculateStartAndEndPoint` (`local.NextPoint`)))
  (bind (_start_2 _end_2) (`self.CalculateStartAndEndPoint` (`self.StartingPoint`)))
  ;[1 1 1] Get corresponding viewpoint
  (bind _issue (`/BcfCommunication/Library/BcfFunctionLibrary.GetFilteredIssue` (`self.IssueIndex`)))
  (bind (_index _guid _topic_guid _image_path _image _location _camera_direction _camera_up_vector _fov _fovh) (break `ViewpointStruct` (`|GetArrayItem` (`.Viewpoints` (break `MarkupStruct` _issue)))))
  (set `local.FovH` _fovh)
  (set `local.FovW` _fov)
  (bind _output_get (set `local.Image` _image))
  (bind _output_get_2 (set `local.PixelWidth` 600))
  (bind _output_get_3 (set `local.PixelHeight` 1280))
  (`self.SetPlaneScaleAndCalcDistance` _output_get_2 _output_get_3)
  (for _index_2 (range 1 (+ (* 600 1280) 1))
    (bind _output_get_4 (set `local.LoopIndex` _index_2))
    (if (== _output_get_4 1)
      ;[1 1 1] First point need to be set indiviually
      (bind _outhit (`KismetSystemLibrary.LineTraceSingle` :`Start` _start_2 :`End` _end_2 :`TraceChannel` "TraceTypeQuery1" :`DrawDebugType` "ForDuration" :`DrawTime` 10.0))
      (set `local.NextPoint` (+ (`self.StartingPoint`) (`KismetMathLibrary.MakeVector` 0.0 (* (`self.WidthDistance`) 100.0))))
      ;[1 1 1] Add Hit Actor if it is a ViewerMeshActor
      (bind _asviewer_mesh_actor (cast `/Game/Viewer/01_Core/Meshes/ViewerMeshActor` (`.HitActor` (`GameplayStatics.BreakHitResult` _outhit))))
      (`KismetArrayLibrary.Array_AddUnique` (`self.VisibleActors`) _asviewer_mesh_actor)
      (else
        ;[1 1 1] Trace Next point
        (bind _outhit_2 (`KismetSystemLibrary.LineTraceSingle` :`Start` _start :`End` _end :`TraceChannel` "TraceTypeQuery1" :`DrawDebugType` "ForDuration" :`DrawTime` 10.0))
        (bind _asviewer_mesh_actor_2 (cast `/Game/Viewer/01_Core/Meshes/ViewerMeshActor` (`.HitActor` (`GameplayStatics.BreakHitResult` _outhit_2)))
          (:`then`
            (`KismetArrayLibrary.Array_AddUnique` (`self.VisibleActors`) _asviewer_mesh_actor_2))
          (:`CastFailed`
            _))
        (if (== (mod (`local.LoopIndex`) 600) 0)
          ;[1 1 1] If true add height difference to first point in row
          (bind _output_get_5 (set `self.StartingPoint` (- (`self.StartingPoint`) (`KismetMathLibrary.MakeVector` 0.0 0.0 (* (`self.HeightDistance`) 100.0)))))
          (set `local.NextPoint` _output_get_5)
          (else
            ;[1 1 1] If false continue to next point in row
            (set `local.NextPoint` (+ (`local.NextPoint`) (`KismetMathLibrary.MakeVector` 0.0 (* (`self.WidthDistance`) 100.0))))))))))

(fn `SetPlaneScaleAndCalcDistance`
  (params (PixelWidth :type Integer) (PixelHeight :type Integer))
  (bind _returnvalue (* PixelHeight 0.001))
  (bind _returnvalue_2 (* PixelWidth 0.001))
  (bind _returnvalue_3 (/ _returnvalue (`KismetMathLibrary.Conv_IntToDouble` PixelHeight)))
  (bind _returnvalue_4 (/ _returnvalue_2 (`KismetMathLibrary.Conv_IntToDouble` PixelWidth)))
  (bind _output_get (set `self.WidthDistance` _returnvalue_4))
  (bind _output_get_2 (set `self.HeightDistance` _returnvalue_3))
  (`SceneComponent.SetRelativeScale3D` (`self.Plane`) (`KismetMathLibrary.MakeVector` _returnvalue _returnvalue_2 1.0))
  (set `self.StartingPoint` (+ (`SceneComponent.RelativeLocation` (`self.Plane`)) (`KismetMathLibrary.MakeVector` 0.0 (+ (* (.y (`KismetMathLibrary.MakeVector` 100.0 (`KismetMathLibrary.Conv_IntToDouble` (/ (/ (`local.PixelWidth`) 10) 2)) (`KismetMathLibrary.Conv_IntToDouble` (/ (/ (`local.PixelHeight`) 10) 2)))) -1.0) (/ _returnvalue_4 2.0)) (- (.z (`KismetMathLibrary.MakeVector` 100.0 (`KismetMathLibrary.Conv_IntToDouble` (/ (/ (`local.PixelWidth`) 10) 2)) (`KismetMathLibrary.Conv_IntToDouble` (/ (/ (`local.PixelHeight`) 10) 2)))) (/ _returnvalue_3 2.0))))))

(fn `ShowHide`
  (params (bShow :type Boolean))
  (`SceneComponent.SetVisibility` (`self.Camera`) bShow false)
  (`PrimitiveComponent.SetCollisionEnabled` (`self.Camera`) (select `bool` bShow :`false` "NoCollision" :`true` "QueryAndPhysics" :!type "ECollisionEnabled Enum")))

(fn `UserConstructionScript`)