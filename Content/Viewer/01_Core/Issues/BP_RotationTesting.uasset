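; BP_RotationTesting is a test actor for converting between Unreal transforms and issue-style viewpoints made of a location, camera direction and up vector.
; CalculateNewRotation passes the actor's location and rotation through CreateViewpointTransform and stores the results in the New variables.
; SetTransform runs the reverse conversion, building a viewpoint from the Original variables and applying GetViewpointTransform's rotation and location to the actor.
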(event `CalculateNewRotation`
  (bind (_viewpointlocation _viewpointcameradirection _viewpointcameraupvector) (`/BcfCommunication/Library/BcfFunctionLibrary.CreateViewpointTransform` (`self.K2_GetActorLocation`) (`self.K2_GetActorRotation`)))
  (set `self.NewDirection` _viewpointcameradirection)
  (set `self.NewUp` _viewpointcameraupvector)
  (set `self.NewLocation` _viewpointlocation))

(event `SetTransform`
  (`self.K2_SetActorRotation` (.rotation (`/BcfCommunication/Library/BcfFunctionLibrary.GetViewpointTransform` (make `ViewpointStruct` 0 "" "" "" null (`self.OriginalLocation`) (`self.OrigininalDirection`) (`self.OriginalUp`)))))
  (`self.K2_SetActorLocation` (.location (`/BcfCommunication/Library/BcfFunctionLibrary.GetViewpointTransform` (make `ViewpointStruct` 0 "" "" "" null (`self.OriginalLocation`) (`self.OrigininalDirection`) (`self.OriginalUp`))))))

(fn `UserConstructionScript`)