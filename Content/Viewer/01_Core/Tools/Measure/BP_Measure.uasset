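; BP_Measure is a one-shot viewer tool that measures the straight-line distance between two clicked points in the scene.
; On spawn it sets a crosshair cursor and removes existing BP_Needle markers.
; A non-looping MultiGate sequences left clicks, each placing a needle at the complex Visibility trace hit under the cursor.
; The second click writes the distance to ProjectSetup's SPDistance and destroys the tool, leaving both needles in place.
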(event `self.ReceiveBeginPlay`
  (`PlayerController.SetMouseCursorWidget` (`GameplayStatics.GetPlayerController` 0) "Crosshairs" null)
  (bind _outactors (`GameplayStatics.GetAllActorsOfClass` "/Game/Viewer/01_Core/Tools/Measure/BP_Needle.BP_Needle_C"))
  (for _array_element _outactors
    (`self.K2_DestroyActor` _array_element)))

(event `Key|LeftMouseButton`
  (params (Key :type "Key Structure"))
  (bind (_bblockinghit _binitialoverlap _time _distance _location) (`GameplayStatics.BreakHitResult` (`PlayerController.GetHitResultUnderCursorByChannel` (`GameplayStatics.GetPlayerController` 0) "TraceTypeQuery1" true)))
  (:`Pressed`
    (`|MultiGate` false
      (:`Out 0`
        (bind _output_get (set `self.FirstLocation` _location))
        (`|SpawnActorFromClass` "/Game/Viewer/01_Core/Tools/Measure/BP_Needle.BP_Needle_C" (`KismetMathLibrary.MakeTransform` _output_get) "Undefined" "OverrideRootScale" null 0 null))
      (:`Out 1`
        (bind _output_get_2 (set `self.SecondLocation` _location))
        (`|SpawnActorFromClass` "/Game/Viewer/01_Core/Tools/Measure/BP_Needle.BP_Needle_C" (`KismetMathLibrary.MakeTransform` _output_get_2) "Undefined" "OverrideRootScale" null 0 null)
        (`SpinBox.SetValue` (`/CAIAViewer/UI/Windows/WBP_PlanSetup.SP_Distance` (`self.ProjectSetup`)) (`KismetMathLibrary.Vector_Distance` (`self.FirstLocation`) (`self.SecondLocation`)))
        (`self.K2_DestroyActor`)))))

(fn `UserConstructionScript`)