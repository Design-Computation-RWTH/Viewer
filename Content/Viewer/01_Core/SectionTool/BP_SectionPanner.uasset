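; BP_SectionPanner is a clickable drag handle for the viewer's section tool that slides along one local axis chosen by Direction.
; Clicking it resets the parent BP_SectionBox and disables pawn input; a left click also opens a Gate that lets Tick apply mouse delta as a local offset.
; A mouse-release event, bound through PC_Viewer, restores pawn input, calls SetBoxEvent on the parent and closes the Gate.
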(event `self.ReceiveBeginPlay`
  (bind _aspc_viewer (cast `/Game/Viewer/01_Core/PC_Viewer` (`GameplayStatics.GetPlayerController` 0)))
  (add `/Game/Viewer/01_Core/PC_Viewer.MouseReleased` _aspc_viewer (`|CreateDelegate` :!event `Released`))
  (`KismetSystemLibrary.PrintString` "Hello"))

(event `self.ReceiveTick`
  (params (DeltaSeconds :type "Float (single-precision)"))
  (bind (_deltax _deltay) (`PlayerController.GetInputMouseDelta` (`GameplayStatics.GetPlayerController` 0)))
  (`/Engine/EditorBlueprintResources/StandardMacros.Gate` true :!label _label
    (:`Exit`
      (`self.K2_AddActorLocalOffset` (select `/Game/Viewer/01_Core/SectionTool/PannerDirection` (`self.Direction`) :`NewEnumerator0` (`KismetMathLibrary.MakeVector` _deltax) :`NewEnumerator2` (`KismetMathLibrary.MakeVector` 0.0 _deltax) :`NewEnumerator4` (`KismetMathLibrary.MakeVector` 0.0 0.0 _deltay))))))

(event `self.SectionBox5.OnClicked`
  (params (TouchedComponent :type "PrimitiveComponent Object Reference") (ButtonPressed :type "Key Structure"))
  (`/Game/Viewer/01_Core/SectionTool/BP_SectionBox.Reset` (cast `/Game/Viewer/01_Core/SectionTool/BP_SectionBox` (`self.GetParentActor`) :!pure true))
  (`self.DisableInput` (`GameplayStatics.GetPlayerPawn` 0) (`GameplayStatics.GetPlayerController` 0))
  (if (== ButtonPressed "LeftMouseButton")
    (goto _label :!via `Open`)))

(event `Released`
  (`self.EnableInput` (`GameplayStatics.GetPlayerPawn` 0) (`GameplayStatics.GetPlayerController` 0))
  (`/Game/Viewer/01_Core/SectionTool/BP_SectionBox.SetBox_Event` (cast `/Game/Viewer/01_Core/SectionTool/BP_SectionBox` (`self.GetParentActor`) :!pure true))
  (goto _label :!via `Close`))

(fn `UserConstructionScript`)