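; Section box actor for the viewer's section tool, sizing a box component and placing panner handles around it on the X, Y and Z axes.
; SetSectionBox fits the box to its child actors' combined bounds and writes center and size to the PC_Data material parameter collection.
; SetBoxExtents instead fits it, with padding, to a supplied actor list.
; DoOnce gates limit box and panner updates until Reset.
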(event `SetPannerGate`
  (`/Engine/EditorBlueprintResources/StandardMacros.DoOnce` false :!label _label
    (:`Completed`
      (`self.SetPanner`))))

(event `Reset`
  (`|ExecutionSequence`
    (:`then_0`
      (goto _label :!via `Reset`))
    (:`then_1`
      (goto _label_2 :!via `Reset`))))

(event `SetBox_Event`
  (`/Engine/EditorBlueprintResources/StandardMacros.DoOnce` false :!label _label_2
    (:`Completed`
      (`self.SetSectionBox`))))

(fn `Set Box Extents`
  (params (Actors :type "Array of Actor Object Reference"))
  (locals (Origin :type "Vector Structure") (Extent :type "Vector Structure"))
  (bind _sectionbox (`self.SectionBox`))
  (bind (_center _boxextent) (`GameplayStatics.GetActorArrayBounds` Actors))
  (set `local.Origin` _center)
  (set `local.Extent` _boxextent)
  (`SceneComponent.K2_SetWorldLocation` _sectionbox (`local.Origin`) false false)
  (`SceneComponent.SetRelativeScale3D` _sectionbox (/ (* (+ (`local.Extent`) 100) 2) 100))
  (`self.SetPanner`))

(fn `SetPanner`
  (locals (Origin :type "Vector Structure" :default (0.0 0.0 0.0)) (Extents :type "Vector Structure" :default (0.0 0.0 0.0)))
  (bind (_origin _boxextent) (`KismetSystemLibrary.GetComponentBounds` (`self.SectionBox`)))
  (set `local.Origin` _origin)
  (set `local.Extents` _boxextent)
  (`SceneComponent.K2_SetWorldLocation` (`self.SP_X`) (+ (`local.Origin`) (`KismetMathLibrary.MakeVector` (+ (.x (`local.Extents`)) 20.0))) false false)
  (`SceneComponent.K2_SetWorldLocation` (`self.SP_-X`) (- (`local.Origin`) (`KismetMathLibrary.MakeVector` (+ (.x (`local.Extents`)) 20.0))) false false)
  (`SceneComponent.K2_SetWorldLocation` (`self.SP_Y`) (+ (`local.Origin`) (`KismetMathLibrary.MakeVector` 0.0 (+ (.y (`local.Extents`)) 20.0))) false false)
  (`SceneComponent.K2_SetWorldLocation` (`self.SP_-Y`) (- (`local.Origin`) (`KismetMathLibrary.MakeVector` 0.0 (+ (.y (`local.Extents`)) 20.0))) false false)
  (`SceneComponent.K2_SetWorldLocation` (`self.SP_Z`) (+ (`local.Origin`) (`KismetMathLibrary.MakeVector` 0.0 0.0 (+ (.z (`local.Extents`)) 20.0))) false false)
  (`SceneComponent.K2_SetWorldLocation` (`self.SP_-Z`) (- (`local.Origin`) (`KismetMathLibrary.MakeVector` 0.0 0.0 (+ 0.0 (.z (`local.Extents`))))) false false))

(fn `SetSectionBox`
  (locals (Origin :type "Vector Structure" :default (0.0 0.0 0.0)) (Extent :type "Vector Structure" :default (0.0 0.0 0.0)) (Panner :type "Array of Actor Object Reference"))
  (bind _sectionbox (`self.SectionBox`))
  (bind (_origin _boxextent) (`KismetSystemLibrary.GetComponentBounds` (`self.SectionBox`)))
  (bind _returnvalue (* (`local.Extent`) 2))
  (`KismetSystemLibrary.DrawDebugBox` _origin _boxextent (struct :`R` 1.0 :`G` 0.120887 :`A` 1.0) (struct) 5.0 10.0)
  (for _array_element (`self.K2_GetComponentsByClass` "/Script/Engine.ChildActorComponent")
    (`KismetArrayLibrary.Array_Add` (`local.Panner`) (`ChildActorComponent.ChildActor` _array_element)))
  (bind (_center _boxextent_2) (`GameplayStatics.GetActorArrayBounds` (`local.Panner`) true))
  ;[1 1 1] Only works when object "grows". Bounds need to be calculated just from Panner, not box
  (set `local.Origin` _center)
  (set `local.Extent` _boxextent_2)
  (`SceneComponent.K2_SetWorldLocation` _sectionbox (`local.Origin`) false false)
  (`SceneComponent.SetRelativeScale3D` _sectionbox (/ _returnvalue 100))
  (`KismetMaterialLibrary.SetVectorParameterValue` "/Game/Viewer/01_Core/SectionTool/MaterialFunction/PC_Data.PC_Data" "Position_1" (`KismetMathLibrary.Conv_VectorToLinearColor` (`local.Origin`)))
  (set `self.Bounds` _returnvalue)
  (`KismetMaterialLibrary.SetVectorParameterValue` "/Game/Viewer/01_Core/SectionTool/MaterialFunction/PC_Data.PC_Data" "Bounds" (`KismetMathLibrary.Conv_VectorToLinearColor` _returnvalue))
  (`self.SetPannerGate`))

(fn `UserConstructionScript`)